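; AudioController_BP manages a single 2D background audio track in the Camera Director Kit.
; ChangeBackGroundAudioClip takes a clip and volume, then swaps the sound on the existing audio component and restarts it, or stops it when the clip is invalid.
; If no component exists yet, it spawns one with SpawnSound2D and keeps the reference for later changes.
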(event EventBeginPlay)

(fn ConstructionScript)

(fn ChangeBackGroundAudioClip
  (params (AudioClip :type Sound%20Cue%20Object%20Reference) (Volume :type Float%20%28single-precision%29))
  (if (Utilities|IsValid (Variables|Default|GetBackGround01_AudioComponent))
    (if (Utilities|IsValid AudioClip)
      (Audio|Components|Audio|SetSound (Variables|Default|GetBackGround01_AudioComponent) AudioClip)
      (Audio|Components|Audio|SetVolumeMultiplier (Variables|Default|GetBackGround01_AudioComponent) Volume :!class /Script/Engine.AudioComponent)
      (Audio|Components|Audio|Play (Variables|Default|GetBackGround01_AudioComponent) 0.0)
      (else
        (Audio|Components|Audio|Stop (Variables|Default|GetBackGround01_AudioComponent))))
    (elif (Utilities|IsValid AudioClip)
      (bind _output_get (Variables|Default|SetBackGround_AudioClip AudioClip))
      (bind _output_get_2 (Variables|Default|SetBackGround_Volume Volume))
      (bind _returnvalue (Audio|SpawnSound2D _output_get _output_get_2 1.0 0.0 0))
      (bind _output_get_3 (Variables|Default|SetBackGround01_AudioComponent _returnvalue))
      (Audio|Components|Audio|Play _output_get_3 0.0))))