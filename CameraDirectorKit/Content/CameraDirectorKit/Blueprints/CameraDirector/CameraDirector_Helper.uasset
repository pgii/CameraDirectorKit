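; Helper function library for the Camera Director kit that finds and drives scene actors by enum-based names.
; Lookups scan all actors of a class, matching characters by a mesh component tag and target points, directors and sockets by name, while splines return the first found.
; Built on these, it starts a director's diagram, changes background audio, overrides animation speed and swaps child-actor classes on character sockets.
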(fn GetCharacterbyTag
  (params (CharacterTag :type CharacterEnum%20Enum :default "NewEnumerator5"))
  (bind _outactors (Actor|GetAllActorsOfClass 0 "/Game/CameraDirectorKit/ThirdPersonBP/Blueprints/ThirdPersonCharacter.ThirdPersonCharacter_C"))
  (for _array_element _outactors
    (if (Components|ComponentHasTag (Variables|/Script/Engine.Character|GetMesh _array_element) (Utilities|String|StringToName (Utilities|String|EnumtoString CharacterTag)))
      (return _array_element true)))
  (return 0 false))

(fn GetTargetPointbyName
  (params (TargetPointName :type TargetPointEnum%20Enum :default "NewEnumerator4"))
  (bind _outactors (Actor|GetAllActorsOfClass 0 "/Script/Engine.TargetPoint"))
  (for _array_element _outactors
    (if (Utilities|Enum|Equal(Enum) (Utilities|GetObjectName _array_element) (Utilities|String|EnumtoString TargetPointName))
      (return _array_element true)))
  (return 0 false))

(fn ChangeBackGroundAudioClip
  (params (AudioClip :type Sound%20Cue%20Object%20Reference) (Volume :type Float%20%28single-precision%29))
  (bind _outactors (Actor|GetAllActorsOfClass 0 "/Game/CameraDirectorKit/Blueprints/AudioController_BP.AudioController_BP_C"))
  (for _array_element _outactors
    (bind _asaudio_controller_bp (Utilities|Casting|CastToAudioController_BP _array_element))
    (Default|ChangeBackGroundAudioClip _asaudio_controller_bp AudioClip Volume)))

(fn GetCharacterSpline
  (bind _outactors (Actor|GetAllActorsOfClass 0 "/Game/CameraDirectorKit/Blueprints/CharacterSpline_BP.CharacterSpline_BP_C"))
  (for _array_element _outactors
    (return _array_element true))
  (return 0 false))

(fn GetCameraDirectorbyName
  (params (CameraDirectorName :type CameraDirectorEnum%20Enum :default "NewEnumerator0"))
  (bind _outactors (Actor|GetAllActorsOfClass 0 "/Game/CameraDirectorKit/Blueprints/CameraDirector/CameraDirector_BP.CameraDirector_BP_C"))
  (for _array_element _outactors
    (if (Utilities|Enum|Equal(Enum) (Utilities|GetDisplayName _array_element) (Utilities|String|EnumtoString CameraDirectorName))
      (return _array_element true)))
  (return 0 false))

(fn SetCharacterManualSpeed
  (params (CharacterName :type CharacterEnum%20Enum :default "NewEnumerator5") (Speed :type Float%20%28single-precision%29) (isSpeedManual :type Boolean))
  (bind (_character _isfound) (CallFunction|GetCharacterbyTag CharacterName))
  (bind _asthird_person_anim_bp (Utilities|Casting|CastToThirdPerson_AnimBP (Components|SkeletalMesh|GetAnimInstance (Variables|/Script/Engine.Character|GetMesh _character))))
  (Variables|/Game/CameraDirectorKit/ThirdPersonBP/Animations/ThirdPerson_AnimBP.ThirdPerson_AnimBP_C|SetisSpeedManual _asthird_person_anim_bp isSpeedManual)
  (Variables|/Game/CameraDirectorKit/ThirdPersonBP/Animations/ThirdPerson_AnimBP.ThirdPerson_AnimBP_C|SetSpeed _asthird_person_anim_bp Speed)
  (return _asthird_person_anim_bp _isfound))

(fn GetCameraCharacterArray
  (params (CharacterName :type CharacterEnum%20Enum :default "NewEnumerator5"))
  (bind (_character _isfound) (CallFunction|GetCharacterbyTag CharacterName))
  (return (Actor|GetComponentsByClass _character "/Script/Engine.CameraComponent") _isfound))

(fn GetCameraSpline
  (bind _outactors (Actor|GetAllActorsOfClass 0 "/Game/CameraDirectorKit/Blueprints/CameraSpline_BP.CameraSpline_BP_C"))
  (for _array_element _outactors
    (return _array_element true))
  (return 0 false))

(fn GetCameraPointbyName
  (params (CameraPointName :type CameraPointEnum%20Enum :default "NewEnumerator4"))
  (bind _outactors (Actor|GetAllActorsOfClass 0 "/Script/Engine.TargetPoint"))
  (for _array_element _outactors
    (if (Utilities|Enum|Equal(Enum) (Utilities|GetObjectName _array_element) (Utilities|String|EnumtoString CameraPointName))
      (return _array_element true)))
  (return 0 false))

(fn StartCameraDirector
  (params (CameraDirectorName :type CameraDirectorEnum%20Enum :default "NewEnumerator0") (Diagram :type Diagram%20Master%20BP%20Class%20Reference))
  (bind (_cameradirector _isfound) (CallFunction|GetCameraDirectorbyName CameraDirectorName))
  (if _isfound
    (Variables|/Game/CameraDirectorKit/Blueprints/CameraDirector/CameraDirector_BP.CameraDirector_BP_C|SetDisplayDiagram _cameradirector Diagram)
    (Default|InitDiagram _cameradirector)
    (return _cameradirector true)
    (else
      (return 0 false))))

(fn SetSocketObject
  (params (CharacterName :type CharacterEnum%20Enum :default "NewEnumerator5") (CharacterSocketName :type CharacterSocketEnum%20Enum :default "NewEnumerator7") (LookAtObject :type Look%20at%20Master%20Object%20Class%20Reference) (CorrectTransform :type Transform))
  (bind (_socketobject _isfound) (CallFunction|GetCharacterSocket CharacterName CharacterSocketName))
  (if _isfound
    (CallFunction|ClearSocketObject CharacterName CharacterSocketName)
    (if (Utilities|IsValidClass LookAtObject)
      (ChildActorComponent|SetChildActorClass _socketobject LookAtObject)
      (Class|SceneComponent|AddLocalTransform (Components|GetChildComponent _socketobject 0) CorrectTransform false false))
    (else
      (Development|PrintString 0 "Socket not found"))))

(fn GetCharacterSocket
  (params (CharacterName :type CharacterEnum%20Enum :default "NewEnumerator5") (CharacterSocketName :type CharacterSocketEnum%20Enum :default "NewEnumerator7"))
  (bind _character (CallFunction|GetCharacterbyTag CharacterName))
  (for _array_element (Actor|GetComponentsByClass _character "/Script/Engine.ChildActorComponent")
    (if (Utilities|Enum|Equal(Enum) (Utilities|GetObjectName _array_element) (Utilities|String|EnumtoString CharacterSocketName))
      (return _array_element true)))
  (return 0 false))

(fn ClearSocketObject
  (params (CharacterName :type CharacterEnum%20Enum :default "NewEnumerator5") (CharacterSocket :type CharacterSocketEnum%20Enum :default "NewEnumerator7"))
  (bind (_socketobject _isfound) (CallFunction|GetCharacterSocket CharacterName CharacterSocket))
  (if _isfound
    (ChildActorComponent|SetChildActorClass _socketobject "/Game/CameraDirectorKit/Props/Master/LookAt_Master_Object.LookAt_Master_Object_C")))