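; Camera director actor that turns fifteen preset camera placements into camera actors and opens a diagram for them.
; InitDiagram spawns a camera at each component's transform into CameraArray, flags this director as current, spawns DisplayDiagram, and enables mouse cursor, Game and UI input, and cinematic mode.
; ResetCameraDirector destroys those cameras and clears the current flag, leaving the diagram and input state untouched.
; The construction script tints all placement arrows with ArrowColor.
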(event Custom|ResetCameraDirector
  (bind _cameraarray (Variables|Default|GetCameraArray))
  (for _array_element _cameraarray
    (Actor|DestroyActor _array_element))
  (Utilities|Array|Clear _cameraarray)
  (Variables|Default|SetisCurrentCameraDirector false))

(event Custom|InitDiagram
  (bind _returnvalue (Game|GetPlayerController 0))
  (for (_array_element _array_index) (Utilities|Array|MakeArray (Variables|Default|GetCamera00) (Variables|Default|GetCamera01) (Variables|Default|GetCamera02) (Variables|Default|GetCamera03) (Variables|Default|GetCamera04) (Variables|Default|GetCamera05) (Variables|Default|GetCamera06) (Variables|Default|GetCamera07) (Variables|Default|GetCamera08) (Variables|Default|GetCamera09) (Variables|Default|GetCamera10) (Variables|Default|GetCamera11) (Variables|Default|GetCamera12) (Variables|Default|GetCamera13) (Variables|Default|GetCamera14))
    (bind _returnvalue_2 (Game|SpawnActorfromClass "/Script/Engine.CameraActor" (Transformation|GetWorldTransform _array_element) "AlwaysSpawn" 0 0))
    (Utilities|Array|Insert (Variables|Default|GetCameraArray) _returnvalue_2 _array_index))
  (Variables|Default|SetisCurrentCameraDirector true)
  (Game|SpawnActorfromClass (Variables|Default|GetDisplayDiagram) (Math|Transform|MakeTransform "0, 0, 0") "AlwaysSpawn" 0 0)
  (Input|SetInputModeGameandUI _returnvalue 0 "DoNotLock" true)
  (Variables|/Script/Engine.PlayerController|SetbShowMouseCursor _returnvalue true)
  (Class|PlayerController|SetCinematicMode _returnvalue true false true true false))

(fn ConstructionScript
  (Components|Arrow|SetArrowColor(LinearColor) (Variables|Default|GetArrowCamera01) (Variables|Default|GetArrowColor)))