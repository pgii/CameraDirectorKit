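; Camera Director Kit diagram that runs the opening demo cutscene and menu.
; On BeginPlay it fades, moves and turns tagged characters to face each other, then blends between character cameras for a greeting subtitle.
; A four-answer question then either fades, ends the diagram and starts the Character, Camera or Effects demo diagram, or simply ends it on Exit.
; The whole sequence is chained through latent completion callbacks.
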(event EventBeginPlay
  (CallFunction|CreateNewDiagram)
  (Utilities|StartFadeOut
    (:Out
      (Utilities|CharacterMoveTargetPoint
        (:Completed
          (Utilities|CharacterRotation "NewEnumerator5" "NewEnumerator0"
            (:Completed
              (Utilities|CharacterMoveTargetPoint "NewEnumerator0" "NewEnumerator21" true 0.0 "-150.000000,0,0" false
                (:Out
                  (Utilities|CharacterMoveTargetPoint :Character "NewEnumerator6" :TargetPoint "NewEnumerator21"
                    (:Completed
                      (Utilities|CharacterFacetoFace "NewEnumerator0" "NewEnumerator6"
                        (:Completed
                          (Utilities|SwitchCameraCharacter self "NewEnumerator6" "NewEnumerator4" "NewEnumerator0" "NewEnumerator2" 1.0 45.0 0.0 false
                            (:BlendTimeFinished
                              (Utilities|NewSubtitle self "Hi!" 0.0 false 1.0 5.0
                                (:ShowTimeFinished
                                  (Utilities|SwitchCameraCharacter self "NewEnumerator0" "NewEnumerator5" "NewEnumerator6" "NewEnumerator2" 0.15 45.0 0.0 false
                                    (:BlendTimeFinished
                                      (Utilities|NewQuestion self "Select action" 0.5 "Character" "Camera" "Effects" "Exit" 0.0
                                        (:AnswerSelect01
                                          (Utilities|StartFadein
                                            (:Completed
                                              (bind _character (CallFunction|GetCharacterbyTag "NewEnumerator5"))
                                              (CallFunction|EndDiagram _character)
                                              (CallFunction|StartCameraDirector "NewEnumerator0" "/Game/CameraDirectorKit/Blueprints/Diagram/Diagram_DemoCharacter_BP.Diagram_DemoCharacter_BP_C"))))
                                        (:AnswerSelect02
                                          (Utilities|StartFadein
                                            (:Completed
                                              (bind _character_2 (CallFunction|GetCharacterbyTag "NewEnumerator5"))
                                              (CallFunction|EndDiagram _character_2)
                                              (CallFunction|StartCameraDirector "NewEnumerator0" "/Game/CameraDirectorKit/Blueprints/Diagram/Diagram_DemoCamera_BP.Diagram_DemoCamera_BP_C"))))
                                        (:AnswerSelect03
                                          (Utilities|StartFadein
                                            (:Completed
                                              (bind _character_3 (CallFunction|GetCharacterbyTag "NewEnumerator5"))
                                              (CallFunction|EndDiagram _character_3)
                                              (CallFunction|StartCameraDirector "NewEnumerator0" "/Game/CameraDirectorKit/Blueprints/Diagram/Diagram_DemoEffect_BP.Diagram_DemoEffect_BP_C"))))
                                        (:AnswerSelect04
                                          (bind _character_4 (CallFunction|GetCharacterbyTag "NewEnumerator5"))
                                          (CallFunction|EndDiagram _character_4))))))))))))))))))))))

(event EventTick
  (params (DeltaSeconds :type Float%20%28single-precision%29))
  (|CallParentFunction DeltaSeconds) ; This node is disabled and will not be called.\nDrag off pins to build functionality.
)

(fn ConstructionScript
  (|CallParentFunction))