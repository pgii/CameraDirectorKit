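; Camera Director Kit demo diagram that showcases effect actions through a looping question menu between two characters.
; On BeginPlay it stages both characters and focuses the camera, then offers Slow motion, Camera fade or Back.
; Slow motion runs a spline camera around a jump animation under time dilation; Camera fade chains colored and audio fades with a title.
; Back fades out and starts the Diagram_DemoStart_BP director.
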(event EventBeginPlay
  (CallFunction|CreateNewDiagram)
  (Utilities|StartFadeOut
    (:Out
      (Utilities|CharacterMoveTargetPoint "NewEnumerator0" "NewEnumerator21" true 0.0 "-150.000000,0,0" false
        (:Out
          (Utilities|CharacterMoveTargetPoint :Character "NewEnumerator6" :TargetPoint "NewEnumerator21"
            (:Completed
              (Utilities|CharacterFacetoFace "NewEnumerator0" "NewEnumerator6"
                (:Completed
                  (Utilities|SwitchCameraCharacter self "NewEnumerator0" "NewEnumerator4" "NewEnumerator6" "NewEnumerator2" 0.0 45.0 0.0 false
                    (:BlendTimeFinished
                      (Utilities|NewQuestion self "Effect actions" 0.5 "Slow motion" "Camera fade" "" "Back" 0.0 :!label _label
                        (:AnswerSelect01
                          ;[0.1469 0.3729 1] Slow motion
                          (Utilities|CharacterMoveTargetPoint "NewEnumerator6" "NewEnumerator0" true 0.0 "0,0,400.000000" true
                            (:Completed
                              (Utilities|ShowPopup self "Slow motion" 3.0
                                (:Out
                                  (Utilities|MoveCameraSpline self "NewEnumerator4" 0.0 45.0 false "NewEnumerator11" "NewEnumerator22" "NewEnumerator23" "NewEnumerator0" "NewEnumerator10" "NewEnumerator11" 5e+03 true "NewEnumerator6" :!label _label_2
                                    (:Out
                                      (Utilities|StartSlowMotion 0.025
                                        (:Out
                                          (Utilities|CharacterPlayAnimation "NewEnumerator6" 0.0 "/Game/CameraDirectorKit/ThirdPersonBP/Animations/ThirdPersonJump_Loop.ThirdPersonJump_Loop" false true true
                                            (:Completed
                                              (goto _label_2 Break))))))
                                    (:Breaked
                                      (Utilities|StopSlowMotion
                                        (:Out
                                          (Utilities|FlowControl|Delay 0.5)
                                          (Utilities|CharacterMoveTargetPoint :Character "NewEnumerator6" :TargetPoint "NewEnumerator21"
                                            (:Completed
                                              (Utilities|CharacterFacetoFace "NewEnumerator0" "NewEnumerator6"
                                                (:Completed
                                                  (Utilities|SwitchCameraCharacter self "NewEnumerator0" "NewEnumerator4" "NewEnumerator6" "NewEnumerator2" 0.15 45.0 0.0 false
                                                    (:BlendTimeFinished
                                                      (goto _label))))))))))))))))
                        (:AnswerSelect02
                          ;[1 0.1374 0.1474] Camera fade
                          (Utilities|ShowPopup self "Camera fade" 3.0
                            (:Out
                              (Utilities|StartFadein :Duration 0.5 :DelayBeforeFinish 0.5
                                (:Completed
                                  (Utilities|FlowControl|Delay 1.0)
                                  (Utilities|StartFadeOut
                                    (:Completed
                                      (Utilities|FlowControl|Delay 1.0)
                                      (Utilities|StartFadein 0.5 0.5 (Utilities|Struct|MakeLinearColor 1.0 0.0 0.0 0.0) true true
                                        (:Completed
                                          (Utilities|FlowControl|Delay 1.0)
                                          (Utilities|StartFadeOut 1.0 0.5 (Utilities|Struct|MakeLinearColor 1.0 0.0 0.0 0.0) true true
                                            (:Completed
                                              (Utilities|FlowControl|Delay 1.0)
                                              (Utilities|StartFadein :Duration 0.5 :DelayBeforeFinish 0.5 :ShouldFadeAudio true
                                                (:Completed
                                                  (Utilities|ShowTitle self "Title" 2.0
                                                    (:Completed
                                                      (Utilities|StartFadeOut :ShouldFadeAudio true
                                                        (:Completed
                                                          (Utilities|CharacterMoveTargetPoint :Character "NewEnumerator6" :TargetPoint "NewEnumerator21" :RotateToMatchTargetPoint false
                                                            (:Completed
                                                              (Utilities|CharacterFacetoFace "NewEnumerator0" "NewEnumerator6"
                                                                (:Completed
                                                                  (Utilities|SwitchCameraCharacter self "NewEnumerator0" "NewEnumerator4" "NewEnumerator6" "NewEnumerator2" 0.15 45.0 0.0 false
                                                                    (:BlendTimeFinished
                                                                      (goto _label))))))))))))))))))))))))
                        (:AnswerSelect04
                          (Utilities|StartFadein
                            (:Completed
                              (bind _character (CallFunction|GetCharacterbyTag "NewEnumerator5"))
                              (CallFunction|EndDiagram _character)
                              (CallFunction|StartCameraDirector "NewEnumerator0" "/Game/CameraDirectorKit/Blueprints/Diagram/Diagram_DemoStart_BP.Diagram_DemoStart_BP_C"))))))))))))))))

(event EventTick
  (params (DeltaSeconds :type Float%20%28single-precision%29))
  (|CallParentFunction DeltaSeconds) ; This node is disabled and will not be called.\nDrag off pins to build functionality.
)

(fn ConstructionScript
  (|CallParentFunction))