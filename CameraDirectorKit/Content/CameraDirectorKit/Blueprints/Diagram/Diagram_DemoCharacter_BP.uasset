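; Camera Director Kit demo diagram that showcases character actions through a question-driven dialogue menu.
; BeginPlay stages two characters face to face, then branches into normal or montage animation, a spline walk, or a tour of character-attached cameras with a socketed smartphone.
; Latent nodes chain moves, fades, popups and camera blends, and most branches loop back to their menu.
; The top-level Back option ends the diagram and launches Diagram_DemoStart_BP.
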(event EventBeginPlay
  (CallFunction|CreateNewDiagram)
  (Utilities|StartFadeOut
    (:Out
      (Utilities|CharacterMoveTargetPoint "NewEnumerator0" "NewEnumerator21" true 0.0 "-150.000000,0,0" false
        (:Out
          (Utilities|CharacterMoveTargetPoint :Character "NewEnumerator6" :TargetPoint "NewEnumerator21"
            (:Completed
              (Utilities|CharacterFacetoFace "NewEnumerator0" "NewEnumerator6"
                (:Completed
                  (Utilities|SwitchCameraCharacter self "NewEnumerator0" "NewEnumerator4" "NewEnumerator6" "NewEnumerator2" 0.0 45.0 0.0 false
                    (:BlendTimeFinished
                      (Utilities|NewQuestion self "Character actions" 0.5 "Character animation" "Walk character spline" "Camera character" "Back" 0.0 :!label _label
                        (:AnswerSelect01
                          ;[1 0 0] Character animation
                          (Utilities|NewQuestion self "" 0.5 "Normal animation" "Montage animation" "" "Back" 0.0 :!label _label_2
                            (:AnswerSelect01
                              (Utilities|StartFadein :Duration 0.5 :DelayBeforeFinish 0.5
                                (:Completed
                                  (Utilities|CharacterMoveTargetPoint :Character "NewEnumerator6" :TargetPoint "NewEnumerator0"
                                    (:Completed
                                      (Utilities|CharacterFacetoFace "NewEnumerator0" "NewEnumerator6"
                                        (:Completed
                                          (Utilities|SwitchCameraCharacter self "NewEnumerator0" "NewEnumerator4" "NewEnumerator0" "NewEnumerator7" 0.0 45.0 0.0 false
                                            (:Out
                                              (Utilities|StartFadeOut
                                                (:Out
                                                  (Utilities|ShowPopup self "Normal animation" 3.0
                                                    (:Out
                                                      (Utilities|NewQuestion self "" 0.5 "" "" "" "Stop" 0.0
                                                        (:Out
                                                          (Utilities|CharacterPlayAnimation "NewEnumerator6" 0.0 "/Game/CameraDirectorKit/ThirdPersonBP/Animations/ThirdPersonRun.ThirdPersonRun" true true true :!label _label_3
                                                            (:Breaked
                                                              _)))
                                                        (:AnswerSelect04
                                                          (goto _label_3 Break))))))))))))))))
                            (:AnswerSelect02
                              (Utilities|StartFadein :Duration 0.5 :DelayBeforeFinish 0.5
                                (:Completed
                                  (Utilities|CharacterMoveTargetPoint :Character "NewEnumerator6" :TargetPoint "NewEnumerator0"
                                    (:Completed
                                      (Utilities|CharacterFacetoFace "NewEnumerator0" "NewEnumerator6"
                                        (:Completed
                                          (Utilities|SwitchCameraCharacter self "NewEnumerator0" "NewEnumerator4" "NewEnumerator0" "NewEnumerator7" 0.0 45.0 0.0 false
                                            (:Out
                                              (Utilities|StartFadeOut
                                                (:Out
                                                  (Utilities|ShowPopup self "Montage animation" 3.0
                                                    (:Out
                                                      (Utilities|CharacterPlayMontageAnimation "NewEnumerator6" "/Game/CameraDirectorKit/ThirdPersonBP/Animations/PhoneLookAt_Idle_Montage.PhoneLookAt_Idle_Montage"
                                                        (:Completed
                                                          _)))))))))))))))
                            (:AnswerSelect04
                              (goto _label)))
                          (Utilities|CharacterMoveTargetPoint :Character "NewEnumerator6" :TargetPoint "NewEnumerator21" :RotateToMatchTargetPoint false
                            (:Completed
                              (Utilities|CharacterFacetoFace "NewEnumerator0" "NewEnumerator6"
                                (:Completed
                                  (Utilities|SwitchCameraCharacter self "NewEnumerator0" "NewEnumerator4" "NewEnumerator6" "NewEnumerator2" 0.15 45.0 0.0 false
                                    (:BlendTimeFinished
                                      (goto _label_2))))))))
                        (:AnswerSelect02
                          ;[0.3466 0.3324 1] Walk character spline
                          (Utilities|StartFadein :Duration 0.5 :DelayBeforeFinish 0.5
                            (:Completed
                              (Utilities|WalkCharacterSpline "NewEnumerator6" "NewEnumerator0" "NewEnumerator10" "NewEnumerator11" "NewEnumerator22" "NewEnumerator0" "NewEnumerator4" 1e+02 1.5e+02
                                (:Out
                                  (Utilities|StartFadeOut
                                    (:Out
                                      (Utilities|ShowPopup self "Walk character spline" 3.0
                                        (:Out
                                          (Utilities|FlowControl|Delay 3.0)
                                          (Utilities|SwitchCameraCharacter self "NewEnumerator6" "NewEnumerator1" "NewEnumerator6" "NewEnumerator7" 3.0 9e+01 0.0 false))))))
                                (:Completed
                                  (Utilities|CharacterMoveTargetPoint :Character "NewEnumerator6" :TargetPoint "NewEnumerator21" :RotateToMatchTargetPoint false
                                    (:Completed
                                      (Utilities|CharacterFacetoFace "NewEnumerator0" "NewEnumerator6"
                                        (:Completed
                                          (Utilities|SwitchCameraCharacter self "NewEnumerator0" "NewEnumerator4" "NewEnumerator6" "NewEnumerator2" 0.15 45.0 0.0 false
                                            (:BlendTimeFinished
                                              (goto _label))))))))))))
                        (:AnswerSelect03
                          ;[0.1973 1 0.3063] Camera character
                          (Utilities|StartFadein :Duration 0.5 :DelayBeforeFinish 0.5
                            (:Completed
                              (Utilities|CharacterPlayAnimation "NewEnumerator6" 0.5 "/Game/CameraDirectorKit/ThirdPersonBP/Animations/PhoneLookAt_Anim.PhoneLookAt_Anim" true true true :!label _label_4
                                (:DelayBeforeFinished
                                  (CallFunction|SetSocketObject "NewEnumerator6" "NewEnumerator1" "/Game/CameraDirectorKit/Props/SmartPhone_BP.SmartPhone_BP_C" (Math|Transform|MakeTransform "3.000000,-4.000000,2.000000" "35.000000,-20.000000,150.000000" "1,1,1"))
                                  (Utilities|SwitchCameraCharacter self "NewEnumerator6" "NewEnumerator2" "NewEnumerator6" "NewEnumerator3" 0.0 45.0 0.0 false
                                    (:Out
                                      (Utilities|StartFadeOut
                                        (:Out
                                          (Utilities|ShowPopup self "Right look at camera" 5.0
                                            (:Completed
                                              (Utilities|StartFadein :Duration 0.5 :DelayBeforeFinish 0.5
                                                (:Completed
                                                  (Utilities|SwitchCameraCharacter self "NewEnumerator6" "NewEnumerator4" "NewEnumerator0" "NewEnumerator2" 0.0 45.0 0.0 false
                                                    (:Out
                                                      (Utilities|StartFadeOut
                                                        (:Out
                                                          (Utilities|ShowPopup self "Right dialog camera" 5.0
                                                            (:Completed
                                                              (Utilities|StartFadein :Duration 0.5 :DelayBeforeFinish 0.5
                                                                (:Completed
                                                                  (Utilities|SwitchCameraCharacter self "NewEnumerator6" "NewEnumerator1" "NewEnumerator0" "NewEnumerator2" 0.0 9e+01 0.0 false
                                                                    (:Out
                                                                      (Utilities|StartFadeOut
                                                                        (:Out
                                                                          (Utilities|ShowPopup self "Back camera" 5.0
                                                                            (:Completed
                                                                              (Utilities|StartFadein :Duration 0.5 :DelayBeforeFinish 0.5
                                                                                (:Completed
                                                                                  (Utilities|SwitchCameraCharacter self "NewEnumerator6" "NewEnumerator5" "NewEnumerator0" "NewEnumerator2" 0.0 45.0 0.0 false
                                                                                    (:Out
                                                                                      (Utilities|StartFadeOut
                                                                                        (:Out
                                                                                          (Utilities|ShowPopup self "Left dialog camera" 5.0
                                                                                            (:Completed
                                                                                              (Utilities|SwitchCameraCharacter self "NewEnumerator0" "NewEnumerator4" "NewEnumerator6" "NewEnumerator2" 0.15 45.0 0.0 false
                                                                                                (:DelayFinished
                                                                                                  (goto _label))))))))))))))))))))))))
                                                    (:DelayFinished
                                                      (CallFunction|SetSocketObject "NewEnumerator6" "NewEnumerator1" "/Game/CameraDirectorKit/Props/Master/LookAt_Master_Object.LookAt_Master_Object_C")
                                                      (goto _label_4 Break))))))))))))))))
                        (:AnswerSelect04
                          (Utilities|StartFadein
                            (:Completed
                              (bind _character (CallFunction|GetCharacterbyTag "NewEnumerator5"))
                              (CallFunction|EndDiagram _character)
                              (CallFunction|StartCameraDirector "NewEnumerator0" "/Game/CameraDirectorKit/Blueprints/Diagram/Diagram_DemoStart_BP.Diagram_DemoStart_BP_C"))))))))))))))))

(event EventTick
  (params (DeltaSeconds :type Float%20%28single-precision%29))
  (|CallParentFunction DeltaSeconds) ; This node is disabled and will not be called.\nDrag off pins to build functionality.
)

(fn ConstructionScript
  (|CallParentFunction))