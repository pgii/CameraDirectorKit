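; Master diagram actor for Camera Director Kit cinematic scenes, with unwired example nodes for camera, character, dialogue, audio and effect actions.
; CreateNewDiagram removes the HUD, takes cameras from the current CameraDirector, ensures its widget exists and destroys other diagram actors.
; Tick keeps the look-at camera aimed at its target character.
; EndDiagram restores HUD, game input and the player's main camera, and resets all directors.
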(event EventTick
  (params (DeltaSeconds :type Float%20%28single-precision%29))
  (CallFunction|CharacterLookatUpdate))

(fn ConstructionScript)

(fn CreateNewDiagram
  (Utilities|FlowControl|Sequence
    (:then_0
      (bind _foundwidgets (Widget|GetAllWidgetsOfClass "/Game/CameraDirectorKit/Blueprints/HUD.HUD_C" true))
      (for _array_element _foundwidgets
        (Widget|RemovefromParent _array_element)))
    (:then_1
      (bind _outactors (Actor|GetAllActorsOfClass "/Game/CameraDirectorKit/Blueprints/CameraDirector/CameraDirector_BP.CameraDirector_BP_C"))
      (for _array_element_2 _outactors
        (if (Variables|/Game/CameraDirectorKit/Blueprints/CameraDirector/CameraDirector_BP.CameraDirector_BP_C|GetisCurrentCameraDirector _array_element_2)
          (Variables|Default|SetCameraArray (Variables|/Game/CameraDirectorKit/Blueprints/CameraDirector/CameraDirector_BP.CameraDirector_BP_C|GetCameraArray _array_element_2))
          (bind _foundwidgets_2 (Widget|GetAllWidgetsOfClass "/Game/CameraDirectorKit/Blueprints/CameraDirector/CameraDirector_Widget_BP.CameraDirector_Widget_BP_C" true :!label _label))
          (if (> (Utilities|Array|Length _foundwidgets_2) 0)
            (Variables|Default|SetCameraDirectorWidget (Utilities|Array|Get(acopy) _foundwidgets_2))
            (bind _outactors_2 (Actor|GetAllActorsOfClass "Diagram_Master_BP_C"))
            (for _array_element_3 _outactors_2
              (if (!= _array_element_3 self)
                (Actor|DestroyActor _array_element_3)))
            (else
              (bind _returnvalue (UserInterface|CreateWidget "/Game/CameraDirectorKit/Blueprints/CameraDirector/CameraDirector_Widget_BP.CameraDirector_Widget_BP_C" (Game|GetPlayerController 0)))
              (UserInterface|Viewport|AddtoViewport _returnvalue 0)
              (goto _label))))))))

(fn CharacterLookatUpdate
  (bind _cameralookat (Variables|Default|GetCameraLookAt))
  (bind _characterlookat (Variables|Default|GetCharacterLookAt))
  (Utilities|IsValid _cameralookat
    (:Is%20Valid
      (Utilities|IsValid _characterlookat
        (:Is%20Valid
          (Transformation|SetWorldRotation _cameralookat (Math|Rotator|FindLookatRotation (+ (Transformation|GetWorldLocation _cameralookat) (Variables|Default|GetCameraLookAtLocationCorrection)) (Transformation|GetActorLocation _characterlookat)) false false))))))

(fn EndDiagram
  (params (PlayerCharacter :type Third%20Person%20Character%20Object%20Reference))
  (bind _returnvalue (Game|GetPlayerController 0))
  (bind _maincamera (Variables|/Game/CameraDirectorKit/ThirdPersonBP/Blueprints/ThirdPersonCharacter.ThirdPersonCharacter_C|GetMainCamera PlayerCharacter))
  (Utilities|FlowControl|Sequence
    (:then_0
      (bind _returnvalue_2 (UserInterface|CreateWidget "/Game/CameraDirectorKit/Blueprints/HUD.HUD_C"))
      (UserInterface|Viewport|AddtoViewport _returnvalue_2 0))
    (:then_1
      (Input|SetInputModeGameOnly (Game|GetPlayerController 0))
      (bind _foundwidgets (Widget|GetAllWidgetsOfClass "/Game/CameraDirectorKit/Blueprints/CameraDirector/CameraDirector_Widget_BP.CameraDirector_Widget_BP_C" true))
      (for _array_element _foundwidgets
        (Widget|RemovefromParent _array_element))
      (Variables|/Script/Engine.PlayerController|SetbShowMouseCursor _returnvalue false)
      (Game|Player|SetViewTargetwithBlend _returnvalue (Components|GetOwner _maincamera) 0.0 "VTBlend_Linear" 0.0 false)
      (for _array_element_2 (Actor|GetComponentsByClass PlayerCharacter "/Script/Engine.CameraComponent")
        (if (== _array_element_2 _maincamera)
          (Components|Activation|SetActive _array_element_2 true false)
          (else
            (Components|Activation|SetActive _array_element_2 false true))))
      (bind _outactors (Actor|GetAllActorsOfClass "/Game/CameraDirectorKit/Blueprints/CameraDirector/CameraDirector_BP.CameraDirector_BP_C"))
      (for _array_element_3 _outactors
        (Default|ResetCameraDirector _array_element_3))
      (Class|PlayerController|SetCinematicMode (Game|GetPlayerController 0) false false true true true))))