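; Camera Director Kit demo diagram that showcases camera actions through a nested question menu: switch, move and spline cameras.
; It stages two characters face to face, then each answer runs a latent node chain with fades, title popups and often a spline-walking character.
; Out, Completed and Break pins sync walks with camera nodes; demos return to their submenu.
; Top-level Back ends the diagram and starts Diagram_DemoStart_BP.
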(event EventBeginPlay
  (CallFunction|CreateNewDiagram)
  (Utilities|StartFadeOut
    (:Out
      (Utilities|CharacterMoveTargetPoint "NewEnumerator0" "NewEnumerator21" true 0.0 "-150.000000,0,0" false
        (:Out
          (Utilities|CharacterMoveTargetPoint :Character "NewEnumerator6" :TargetPoint "NewEnumerator21"
            (:Completed
              (Utilities|CharacterFacetoFace "NewEnumerator0" "NewEnumerator6"
                (:Completed
                  (Utilities|SwitchCameraCharacter self "NewEnumerator0" "NewEnumerator4" "NewEnumerator6" "NewEnumerator2" 0.0 45.0 0.0 false
                    (:BlendTimeFinished
                      (Utilities|NewQuestion self "Camera actions" 0.5 "Switch camera" "Move camera" "Camera spline" "Back" 0.0 :!label _label
                        (:AnswerSelect01
                          (Utilities|NewQuestion self "Switch camera" 0.5 "Switch camera view" "Сamera look at" "Custom change view" "Back" 0.0 :!label _label_2
                            (:AnswerSelect01
                              ;[1 0.003125 0.003125] Switch camera view
                              (Utilities|StartFadein :Duration 0.5 :DelayBeforeFinish 0.5
                                (:Completed
                                  (Utilities|WalkCharacterSpline "NewEnumerator6" "NewEnumerator0" "NewEnumerator10" "NewEnumerator11" "NewEnumerator22" "NewEnumerator23" "NewEnumerator0" 1e+02 1.5e+02 :!label _label_3
                                    (:Out
                                      (Utilities|StartFadeOut
                                        (:Out
                                          (Utilities|ShowPopup self "Switch camera view" 3.0
                                            (:Out
                                              (Utilities|SwitchCameraView self "NewEnumerator4" 0.0 45.0 0.0 false false "NewEnumerator5"
                                                (:BlendTimeFinished
                                                  (Utilities|FlowControl|Delay 2.0)
                                                  (Utilities|SwitchCameraView self "NewEnumerator11" 0.0 6e+01 0.0 false false "NewEnumerator5"
                                                    (:BlendTimeFinished
                                                      (Utilities|FlowControl|Delay 2.0)
                                                      (Utilities|SwitchCameraView self "NewEnumerator22" 5.0 9e+01 0.0 false false "NewEnumerator5"
                                                        (:BlendTimeFinished
                                                          (Utilities|FlowControl|Delay 2.0)
                                                          (Utilities|StartFadein
                                                            (:Completed
                                                              (goto _label_3 Break))))))))))))))
                                    (:Breaked
                                      (Utilities|StartFadeOut
                                        (:DelayFinished
                                          (Utilities|CharacterMoveTargetPoint :Character "NewEnumerator6" :TargetPoint "NewEnumerator21" :RotateToMatchTargetPoint false
                                            (:Completed
                                              (Utilities|CharacterFacetoFace "NewEnumerator0" "NewEnumerator6"
                                                (:Completed
                                                  (Utilities|SwitchCameraCharacter self "NewEnumerator0" "NewEnumerator4" "NewEnumerator6" "NewEnumerator2" 0.15 45.0 0.0 false
                                                    (:BlendTimeFinished
                                                      (goto _label_2))))))))))))))
                            (:AnswerSelect02
                              ;[0.1939 0.3743 1] Сamera look at
                              (Utilities|StartFadein :Duration 0.5 :DelayBeforeFinish 0.5
                                (:Completed
                                  (Utilities|WalkCharacterSpline "NewEnumerator6" "NewEnumerator0" "NewEnumerator10" "NewEnumerator11" "NewEnumerator22" "NewEnumerator23" "NewEnumerator0" 1e+02 1.5e+02
                                    (:Out
                                      (Utilities|StartFadeOut
                                        (:Out
                                          (Utilities|ShowPopup self "Сamera look at" 3.0
                                            (:Out
                                              (Utilities|SwitchCameraView self "NewEnumerator22" 0.0 45.0 0.0 false true "NewEnumerator6" :!label _label_4
                                                (:Breaked
                                                  (Utilities|StartFadeOut
                                                    (:DelayFinished
                                                      (Utilities|CharacterMoveTargetPoint :Character "NewEnumerator6" :TargetPoint "NewEnumerator21" :RotateToMatchTargetPoint false
                                                        (:Completed
                                                          (Utilities|CharacterFacetoFace "NewEnumerator0" "NewEnumerator6"
                                                            (:Completed
                                                              (Utilities|SwitchCameraCharacter self "NewEnumerator0" "NewEnumerator4" "NewEnumerator6" "NewEnumerator2" 0.15 45.0 0.0 false
                                                                (:BlendTimeFinished
                                                                  (goto _label_2))))))))))))))))
                                    (:Completed
                                      (Utilities|StartFadein :Duration 0.5 :DelayBeforeFinish 0.5
                                        (:Completed
                                          (goto _label_4 Break))))))))
                            (:AnswerSelect03
                              ;[0 1 0.2652] Custom change view
                              (Utilities|StartFadein :Duration 0.5 :DelayBeforeFinish 0.5
                                (:Completed
                                  (Utilities|SwitchCustomChangeView self true "NewEnumerator4" 45.0 "NewEnumerator0" 45.0 "NewEnumerator11" 45.0 "NewEnumerator22" 45.0 false :!label _label_5
                                    (:Out
                                      (Utilities|WalkCharacterSpline "NewEnumerator6" "NewEnumerator0" "NewEnumerator10" "NewEnumerator11" "NewEnumerator22" "NewEnumerator23" "NewEnumerator0" 1e+02 1.5e+02 :!label _label_6
                                        (:Out
                                          (Utilities|StartFadeOut
                                            (:Out
                                              (Utilities|ShowPopup self "Custom change view" 3.0))))
                                        (:Completed
                                          (goto _label_5 Break))
                                        (:Breaked
                                          (goto _label_5 Break))))
                                    (:Next
                                      (goto _label_6 Break))
                                    (:Breaked
                                      (Utilities|CharacterMoveTargetPoint :Character "NewEnumerator6" :TargetPoint "NewEnumerator21" :RotateToMatchTargetPoint false
                                        (:Completed
                                          (Utilities|CharacterFacetoFace "NewEnumerator0" "NewEnumerator6"
                                            (:Completed
                                              (Utilities|SwitchCameraCharacter self "NewEnumerator0" "NewEnumerator4" "NewEnumerator6" "NewEnumerator2" 0.15 45.0 0.0 false
                                                (:BlendTimeFinished
                                                  (goto _label_2))))))))))))
                            (:AnswerSelect04
                              (goto _label))))
                        (:AnswerSelect02
                          (Utilities|NewQuestion self "Move camera" 0.5 "Zoom camera" "Focus bone camera" "" "Back" 0.0 :!label _label_7
                            (:AnswerSelect01
                              ;[1 0.8675 0] Zoom camera
                              (Utilities|StartFadein :Duration 0.5 :DelayBeforeFinish 0.5
                                (:Completed
                                  (Utilities|CharacterMoveTargetPoint :Character "NewEnumerator6" :TargetPoint "NewEnumerator0" :RotateToMatchTargetPoint false
                                    (:Completed
                                      (Utilities|CharacterFacetoFace "NewEnumerator0" "NewEnumerator6"
                                        (:Completed
                                          (Utilities|SwitchCameraCharacter self "NewEnumerator0" "NewEnumerator4" "NewEnumerator6" "NewEnumerator2" 0.0 45.0 0.0 false
                                            (:BlendTimeFinished
                                              (Utilities|StartFadeOut
                                                (:Out
                                                  (Utilities|ShowPopup self "Zoom camera" 3.0
                                                    (:Out
                                                      (Utilities|ZoomCameraView self "NewEnumerator4" 45.0 9e+01 1e+01 0.0 false
                                                        (:Completed
                                                          (Utilities|FlowControl|Delay 2.0)
                                                          (Utilities|ZoomCameraView self "NewEnumerator4" 9e+01 45.0 1e+01 0.0 false
                                                            (:Completed
                                                              (Utilities|CharacterMoveTargetPoint :Character "NewEnumerator6" :TargetPoint "NewEnumerator21" :RotateToMatchTargetPoint false
                                                                (:Completed
                                                                  (Utilities|CharacterFacetoFace "NewEnumerator0" "NewEnumerator6"
                                                                    (:Completed
                                                                      (Utilities|SwitchCameraCharacter self "NewEnumerator0" "NewEnumerator4" "NewEnumerator6" "NewEnumerator2" 0.15 45.0 0.0 false
                                                                        (:BlendTimeFinished
                                                                          (goto _label_7))))))))))))))))))))))))
                            (:AnswerSelect02
                              ;[0.5981 0 1] Focus bone camera
                              (Utilities|StartFadein :Duration 0.5 :DelayBeforeFinish 0.5
                                (:Completed
                                  (Utilities|CharacterMoveTargetPoint :Character "NewEnumerator6" :TargetPoint "NewEnumerator0" :RotateToMatchTargetPoint false
                                    (:Completed
                                      (Utilities|CharacterFacetoFace "NewEnumerator0" "NewEnumerator6"
                                        (:Completed
                                          (Utilities|SwitchCameraCharacter self "NewEnumerator0" "NewEnumerator5" "NewEnumerator6" "NewEnumerator2" 0.0 45.0 0.0 false
                                            (:BlendTimeFinished
                                              (Utilities|StartFadeOut
                                                (:Out
                                                  (Utilities|ShowPopup self "Focus bone camera" 3.0
                                                    (:Out
                                                      (Utilities|FocusBoneCameraView self "NewEnumerator4" 45.0 false "NewEnumerator6" "NewEnumerator0" "NewEnumerator2" 5.0 0.0 false
                                                        (:Completed
                                                          (Utilities|FlowControl|Delay 2.0)
                                                          (Utilities|FocusBoneCameraView self "NewEnumerator4" 45.0 false "NewEnumerator6" "NewEnumerator2" "NewEnumerator0" 5.0 0.0 true
                                                            (:Completed
                                                              (Utilities|CharacterMoveTargetPoint :Character "NewEnumerator6" :TargetPoint "NewEnumerator21" :RotateToMatchTargetPoint false
                                                                (:Completed
                                                                  (Utilities|CharacterFacetoFace "NewEnumerator0" "NewEnumerator6"
                                                                    (:Completed
                                                                      (Utilities|SwitchCameraCharacter self "NewEnumerator0" "NewEnumerator4" "NewEnumerator6" "NewEnumerator2" 0.15 45.0 0.0 false
                                                                        (:BlendTimeFinished
                                                                          (goto _label_7))))))))))))))))))))))))
                            (:AnswerSelect04
                              (goto _label))))
                        (:AnswerSelect03
                          (Utilities|NewQuestion self "Camera spline" 0.5 "Camera spline" "Camera spline look at" "" "Back" 0.0 :!label _label_8
                            (:AnswerSelect01
                              ;[1 0.1566 0] Camera spline
                              (Utilities|ShowPopup self "Camera spline" 3.0
                                (:Out
                                  (Utilities|MoveCameraSpline self "NewEnumerator4" 2.0 9e+01 false "NewEnumerator0" "NewEnumerator10" "NewEnumerator11" "NewEnumerator22" "NewEnumerator23" "NewEnumerator4" 3e+02 false "NewEnumerator6" :!label _label_9
                                    (:Completed
                                      (Utilities|CharacterMoveTargetPoint :Character "NewEnumerator6" :TargetPoint "NewEnumerator21" :RotateToMatchTargetPoint false
                                        (:Completed
                                          (Utilities|CharacterFacetoFace "NewEnumerator0" "NewEnumerator6"
                                            (:Completed
                                              (Utilities|SwitchCameraCharacter self "NewEnumerator0" "NewEnumerator4" "NewEnumerator6" "NewEnumerator2" 0.15 45.0 0.0 false
                                                (:BlendTimeFinished
                                                  (goto _label_9 Break))))))))
                                    (:Breaked
                                      (goto _label_8))))))
                            (:AnswerSelect02
                              ;[1 0.1566 0] Camera spline look at
                              (Utilities|ShowPopup self "Camera spline look at" 3.0
                                (:Out
                                  (Utilities|WalkCharacterSpline "NewEnumerator6" "NewEnumerator0" "NewEnumerator10" "NewEnumerator11" "NewEnumerator22" "NewEnumerator23" "NewEnumerator0" 1e+02 1.5e+02
                                    (:Out
                                      (Utilities|MoveCameraSpline self "NewEnumerator4" 0.0 45.0 false "NewEnumerator0" "NewEnumerator10" "NewEnumerator11" "NewEnumerator22" "NewEnumerator23" "NewEnumerator4" 1.9e+02 true "NewEnumerator6" :!label _label_10
                                        (:Completed
                                          (Utilities|CharacterMoveTargetPoint :Character "NewEnumerator6" :TargetPoint "NewEnumerator21" :RotateToMatchTargetPoint false
                                            (:Completed
                                              (Utilities|CharacterFacetoFace "NewEnumerator0" "NewEnumerator6"
                                                (:Completed
                                                  (Utilities|SwitchCameraCharacter self "NewEnumerator0" "NewEnumerator4" "NewEnumerator6" "NewEnumerator2" 0.15 45.0 0.0 false
                                                    (:BlendTimeFinished
                                                      (goto _label_8))))))))))
                                    (:Completed
                                      (goto _label_10 Break))))))
                            (:AnswerSelect04
                              (goto _label))))
                        (:AnswerSelect04
                          (Utilities|StartFadein
                            (:Completed
                              (bind _character (CallFunction|GetCharacterbyTag "NewEnumerator5"))
                              (CallFunction|EndDiagram _character)
                              (CallFunction|StartCameraDirector "NewEnumerator0" "/Game/CameraDirectorKit/Blueprints/Diagram/Diagram_DemoStart_BP.Diagram_DemoStart_BP_C"))))))))))))))))

(event EventTick
  (params (DeltaSeconds :type Float%20%28single-precision%29))
  (|CallParentFunction DeltaSeconds) ; This node is disabled and will not be called.\nDrag off pins to build functionality.
)

(fn ConstructionScript
  (|CallParentFunction))