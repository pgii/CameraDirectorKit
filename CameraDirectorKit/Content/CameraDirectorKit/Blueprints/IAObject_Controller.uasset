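; Interaction controller that finds the object the player is looking at and forwards interaction input to it.
; Each tick it runs a short visibility trace from the camera, storing hit actor and component when the component is tagged IAObject.
; The target clears on a miss, while the pawn moves, or while BreakInteraction is set.
; The Interaction input calls CallCharacterInteractionClick only if the target casts to ThirdPersonCharacter.
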(event Custom|CheckInteractionObject
  (bind _returnvalue (Game|GetPlayerCameraManager 0))
  (bind _returnvalue_2 (Transformation|GetActorLocation _returnvalue))
  (if (Variables|Default|GetBreakInteraction)
    (Variables|Default|SetCurrentInteractionObject 0 :!label _label)
    (else
      (|CheckCharacterMove
        (:true
          (goto _label))
        (:false
          (bind (_outhit _returnvalue_3) (Collision|LineTraceByChannel _returnvalue_2 (+ _returnvalue_2 (* (Transformation|GetActorForwardVector _returnvalue) 2.2e+02)) "TraceTypeQuery1" false (Utilities|Array|MakeArray (Game|GetPlayerCharacter 0)) "None"))
          (if _returnvalue_3
            (if (Components|ComponentHasTag (.HitComponent (Collision|BreakHitResult _outhit)) "IAObject")
              (Variables|Default|SetCurrentInteractionObject (.HitActor (Collision|BreakHitResult _outhit)))
              (Variables|Default|SetActiveComponent (.HitComponent (Collision|BreakHitResult _outhit)))
              (else
                (Variables|Default|SetCurrentInteractionObject 0 :!label _label_2)))
            (else
              (goto _label_2))))))))

(event EventTick
  (params (DeltaSeconds :type Float%20%28single-precision%29))
  (CallFunction|CheckInteractionObject))

(event EventBeginPlay)

(event Input|ActionEvents|InputActionInteraction
  (params (Key :type Key%20Structure))
  (:Pressed
    (bind _asthird_person_character (Utilities|Casting|CastToThirdPersonCharacter (Variables|Default|GetCurrentInteractionObject)))
    (Default|CallCharacterInteractionClick _asthird_person_character)))

(fn ConstructionScript)